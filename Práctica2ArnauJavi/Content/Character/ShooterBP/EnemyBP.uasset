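; EnemyBP is an enemy character that damages the hero on contact and awards score when killed.
; Overlapping DamageVolume with HeroBP starts a looping timer that calls AffectHealth on the hero at the attack rate until overlap ends.
; Its own AffectHealth recalculates and prints health.
; On death it ignores WorldDynamic and Pawn collision, increments GameModeTecnoCampus score, detaches its controller and destroys itself after a delay.
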(event OnComponentBeginOverlap(DamageVolume)
  (params (OverlappedComponent :type Primitive%20Component%20Object%20Reference) (OtherActor :type Actor%20Object%20Reference) (OtherComp :type Primitive%20Component%20Object%20Reference) (OtherBodyIndex :type Integer) (bFromSweep :type Boolean) (SweepResult :type Hit%20Result%20Structure%20%28by%20ref%29))
  (bind _ashero_bp (Utilities|Casting|CastToHeroBP OtherActor))
  (Variables|Default|SetHero _ashero_bp)
  (Utilities|Time|SetTimerbyFunctionName 0 "DamageHero" (/ 1.0 (Variables|Default|GetatackPerSecond)) true))

(event OnComponentEndOverlap(DamageVolume)
  (params (OverlappedComponent :type Primitive%20Component%20Object%20Reference) (OtherActor :type Actor%20Object%20Reference) (OtherComp :type Primitive%20Component%20Object%20Reference) (OtherBodyIndex :type Integer))
  (if (== OtherActor (Variables|Default|GetHero))
    (Utilities|Time|ClearTimerbyFunctionName 0 "DamageHero")))

(event Custom|DamageHero
  ;[1 1 1] AffectHealthHero
  (Default|AffectHealth (Variables|Default|GetHero) (Variables|Default|GetDamgedone)))

(event EventAffectHealth
  (params (Value :type Float%20%28single-precision%29))
  (bind _capsulecomponent (Variables|Default|GetCapsuleComponent))
  ;[1 1 1] AffectHealth
  (CallFunction|CalculateHealth Value)
  (Development|PrintString (Utilities|String|ToString(Float) (Variables|Default|GetHealth)) true true "(R=1.000000,G=0.000000,B=0.104621,A=1.000000)")
  (if (Variables|Default|GetisDead)
    (Collision|SetCollisionResponsetoChannel _capsulecomponent "ECC_WorldDynamic" "ECR_Ignore")
    (Collision|SetCollisionResponsetoChannel _capsulecomponent "ECC_Pawn" "ECR_Ignore")
    (bind _asgame_mode_tecno_campus (Utilities|Casting|CastToGameModeTecnoCampus (Game|GetGameMode)))
    (Default|IncrementScore _asgame_mode_tecno_campus 500)
    (Class|Pawn|DetachfromControllerPendingDestroy)
    (Utilities|FlowControl|Delay 3.0)
    (Actor|DestroyActor)))

(fn ConstructionScript
  (|CallParentFunction))